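; TrackedVehicleIHUD is a Blueprint interface through which a HUD reads drivetrain telemetry from a tracked vehicle.
; It declares getters for speed, gear state with reverse and automatic gearbox flags, engine RPM and torque, throttle, and left and right drive values.
; A separate getter supplies a color for the RPM readout.
; The functions carry no logic here and return only default values.
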(fn `HUDGetDriveTLeft`
  (returns (DriveTorque :type "Float (double-precision)"))
  (return 0.0))

(fn `HUDGetDriveTRight`
  (returns (DriveTorque :type "Float (double-precision)"))
  (return 0.0))

(fn `HUDGetEngineRPMColor`
  (returns (Color :type "LinearColor Structure"))
  (return))

(fn `HUDGetEngineTorque`
  (returns (EngineT :type "Float (double-precision)"))
  (return 0.0))

(fn `HUDGetEnigineRPM`
  (returns (EngineRPM :type "Float (double-precision)"))
  (return 0.0))

(fn `HUDGetGear`
  (returns (GearIndex :type Integer) (ReverseGear :type Boolean) (AutoGearBox :type Boolean))
  (return 0 false false))

(fn `HUDGetThrottle`
  (returns (Throttle :type "Float (double-precision)"))
  (return 0.0))

(fn `HUDGetVehicleSpeed`
  (returns (Speed :type "Float (double-precision)"))
  (return 0.0))